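; BP_Hero is the player hero, with data-table-driven class and armor, and opens the character customization widget on BeginPlay.
; CalculateTotalStats sums max HP and mana from the selected class and equipped armor rows into TotalStats.
; UpdateVisual, not called within this Blueprint, sets the body sprite from the class's scene row.
; It also clears the armor sprite slots and fills the one matching the item's position type.
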(event EventBeginPlay
  (CallFunction|CalculateTotalStats)
  (bind _returnvalue (UserInterface|CreateWidget "/Game/DataTabllesUI/Blueprints/UI/WBP_CharacterCustomization.WBP_CharacterCustomization_C" 0 self))
  (UserInterface|Viewport|AddtoViewport _returnvalue 0))

(fn ConstructionScript)

(fn CalculateTotalStats
  (CallFunction|ClearResultStats)
  (CallFunction|AddDatatoResultStats (Variables|DT|GetDT_Classes) (Variables|Selected|GetSelectedClass))
  (CallFunction|AddDatatoResultStats (Variables|DT|GetDT_Items) (Variables|Selected|GetEquippedArmor))
  (Variables|Stats|SetTotalStats (Variables|Stats|GetResultStats)))

(fn AddDatatoResultStats
  (params (DataTable :type Data%20Table%20Object%20Reference) (DataName :type Name))
  (bind _returnvalue (Utilities|GetDataTableRow DataTable DataName)
    (:then
      (Variables|Stats|SetResultStats (Utilities|Struct|MakeST_CharacterStats (+ (.MaxHP (Utilities|Struct|BreakST_CharacterStats _returnvalue)) (.MaxHP (Utilities|Struct|BreakST_CharacterStats (Variables|Stats|GetResultStats)))) (+ (.MaxMana (Utilities|Struct|BreakST_CharacterStats _returnvalue)) (.MaxMana (Utilities|Struct|BreakST_CharacterStats (Variables|Stats|GetResultStats)))))))))

(fn ClearResultStats
  (Variables|Stats|SetResultStats (Utilities|Struct|MakeST_CharacterStats)))

(fn UpdateVisual
  (Visual|UpdateCharacterVisual)
  (Visual|UpdateItemVisual))

(fn UpdateCharacterVisual
  (bind _body (Variables|Default|GetBody))
  (bind _returnvalue (Utilities|GetDataTableRow (Variables|DT|GetDT_CharactersOnScene) (Variables|Selected|GetSelectedClass))
    (:then
      (if (!= (Utilities|Struct|BreakST_Character _returnvalue) _body)
        (Rendering|Components|Sprite|SetSprite _body (Utilities|Struct|BreakST_Character _returnvalue))))))

(fn UpdateItemVisual
  (bind _returnvalue (Utilities|GetDataTableRow (Variables|DT|GetDT_ItemsOnScene) (Variables|Selected|GetEquippedArmor))
    (:then
      (Utilities|FlowControl|Sequence
        (:then_0
          (Visual|ClearItemsVisual))
        (:then_1
          (switch Utilities|FlowControl|Switch|SwitchonF_ItemPosition (.ItemPositionType (Utilities|Struct|BreakST_CharacterItem _returnvalue))
            (:NewEnumerator0
              (Rendering|Components|Sprite|SetSprite (Variables|Default|GetWingArmorSprite) (.ItemSprite (Utilities|Struct|BreakST_CharacterItem _returnvalue))))
            (:NewEnumerator1
              (Rendering|Components|Sprite|SetSprite (Variables|Default|GetEyeArmorSprite) (.ItemSprite (Utilities|Struct|BreakST_CharacterItem _returnvalue))))
            (:NewEnumerator2
              (Rendering|Components|Sprite|SetSprite (Variables|Default|GetTopOfWingArmorSprite) (.ItemSprite (Utilities|Struct|BreakST_CharacterItem _returnvalue))))
            (:NewEnumerator3
              (Rendering|Components|Sprite|SetSprite (Variables|Default|GetFromTheSide) (.ItemSprite (Utilities|Struct|BreakST_CharacterItem _returnvalue))))))))))

(fn ClearItemsVisual
  (Rendering|Components|Sprite|SetSprite (Variables|Default|GetEyeArmorSprite) 0)
  (Rendering|Components|Sprite|SetSprite (Variables|Default|GetTopOfWingArmorSprite) 0)
  (Rendering|Components|Sprite|SetSprite (Variables|Default|GetWingArmorSprite) 0)
  (Rendering|Components|Sprite|SetSprite (Variables|Default|GetFromTheSide) 0))